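; Player controller that opens the lobby UI for the local player and handles look and move input.
; On BeginPlay it adds the Enhanced Input mapping context, creates the lobby widget and shows the cursor in game-and-UI input mode.
; Look input drives yaw and inverted pitch, while move input follows control rotation.
; Both input handlers act on player pawn index 0 rather than the controller's own pawn.
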(event Input|EnhancedActionEvents|EnhancedInputActionIA_Look
  (params (ActionValue :type Vector%202D%20Structure) (ElapsedSeconds :type Float%20%28double-precision%29) (TriggeredSeconds :type Float%20%28double-precision%29) (InputAction :type Input%20Action%20Object%20Reference :default "/Game/Blueprints/Player/Input/IA_Look.IA_Look"))
  (bind (_x _y) (Math|Vector2D|BreakVector2D ActionValue))
  (bind _returnvalue (Game|Player|GetPlayerPawn 0))
  (Pawn|Input|AddControllerYawInput _returnvalue _x)
  (Pawn|Input|AddControllerPitchInput _returnvalue (* _y -1.0)))

(event Input|EnhancedActionEvents|EnhancedInputActionIA_Move
  (params (ActionValue :type Vector%202D%20Structure) (ElapsedSeconds :type Float%20%28double-precision%29) (TriggeredSeconds :type Float%20%28double-precision%29) (InputAction :type Input%20Action%20Object%20Reference :default "/Game/Blueprints/Player/Input/IA_Move.IA_Move"))
  (bind (_x _y) (Math|Vector2D|BreakVector2D ActionValue))
  (bind _returnvalue (Game|Player|GetPlayerPawn 0))
  (bind _returnvalue_2 (Game|Player|GetPlayerPawn 0))
  (bind _returnvalue_3 (Pawn|GetControlRotation _returnvalue :!class /Script/Engine.Pawn))
  (Pawn|Input|AddMovementInput _returnvalue (Math|Vector|GetRightVector (Math|Rotator|MakeRotator (.roll _returnvalue_3) 0.0 (.yaw _returnvalue_3))) _x false)
  (Pawn|Input|AddMovementInput _returnvalue_2 (Math|Vector|GetForwardVector (Math|Rotator|MakeRotator 0.0 0.0 (.yaw (Pawn|GetControlRotation _returnvalue_2 :!class /Script/Engine.Pawn)))) _y false))

(event EventBeginPlay
  (bind _returnvalue (PlayerController|LocalPlayerSubsystems|GetEnhancedInputLocalPlayerSubsystem))
  (if (Pawn|IsLocalPlayerController)
    (Utilities|IsValid _returnvalue
      (:Is%20Valid
        (Input|AddMappingContext _returnvalue "/Game/Blueprints/Player/Input/IMC_Player.IMC_Player" 0 "(bIgnoreAllPressedKeysUntilRelease=True,bForceImmediately=False,bNotifyUserSettings=False)")
        (bind _returnvalue_2 (UserInterface|CreateWidget "/Game/Blueprints/Lobby/WBP_LobbyUI.WBP_LobbyUI_C"))
        (Variables|Default|SetLobbyUI _returnvalue_2)
        (UserInterface|Viewport|AddtoViewport _returnvalue_2 0)
        (Variables|Default|SetbShowMouseCursor true)
        (Input|SetInputModeGameandUI self 0 "DoNotLock" true false)))))

(fn ConstructionScript)