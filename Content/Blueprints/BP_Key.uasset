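; BP_Key is an interactable key item that can always be interacted with and always reports itself as edible.
; Interact calls the MC_TransferItem event, which passes the key to the GameState through TransferItemMessage, leaving the transfer itself to the GameState.
; Its query functions expose the Cube component and its mesh, and make interaction instant with no cooldown.
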(event Custom|MC_TransferItem
  (Class|BPIGameState|TransferItem(Message) (Game|GetGameState) self))

(event EventInteract
  (params (Interactor :type Actor%20Object%20Reference) (Role :type E_Roles%20Enum :default "NewEnumerator0"))
  (CallFunction|MCTransferItem))

(fn ConstructionScript)

(fn CanbeEaten?
  (return true))

(fn CanInteract?
  (return true))

(fn GetMesh
  (bind _cube (Variables|Default|GetCube))
  (return (Variables|/Script/Engine.StaticMeshComponent|GetStaticMesh _cube) _cube))

(fn InteractCooldown
  (return 0.0))

(fn InteractTime
  (return 0.0))