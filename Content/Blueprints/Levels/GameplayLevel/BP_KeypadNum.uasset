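; BP_KeypadNum is a single interactable number key for a keypad in the gameplay level.
; On BeginPlay it pushes its Num value into the WBP_DisplayNumber shown by its widget component.
; Interact goes through MC_Interact, apparently a multicast, which fires the OnKeyPressed dispatcher with Num for listeners to handle.
; Its interaction functions report it as always interactable, never edible, with no hold time or cooldown.
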(event Custom|MC_Interact
  (Default|CallOnKeyPressed (Variables|Default|GetNum)))

(event EventBeginPlay
  (bind _aswbp_display_number (Utilities|Casting|CastToWBP_DisplayNumber (UserInterface|GetWidget (Variables|Default|GetWidget))))
  (Default|SetNumber _aswbp_display_number (Variables|Default|GetNum)))

(event EventInteract
  (params (Interactor :type Actor%20Object%20Reference) (Role :type E_Roles%20Enum :default "NewEnumerator0"))
  (CallFunction|MCInteract))

(fn ConstructionScript)

(fn CanbeEaten?
  (return false))

(fn CanInteract?
  (return true))

(fn GetMesh
  (return 0 0))

(fn InteractCooldown
  (return 0.0))

(fn InteractTime
  (return 0.0))