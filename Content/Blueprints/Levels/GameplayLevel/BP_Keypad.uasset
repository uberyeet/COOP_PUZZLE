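; BP_Keypad is an in-level numeric keypad that opens the end door when the correct code is entered.
; On BeginPlay it binds to the key-press dispatcher of ten BP_KeypadNum child actors, appending each digit to a string shown on a WBP_DisplayNumber widget.
; At four digits it compares the integer value with BP_PuzzleGameplay's DisplayNumber, opening the door on a match or clearing the entry otherwise.
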(event Custom|OnKeyPressed_Event
  (params (Num :type Integer))
  (bind _returnvalue (Utilities|String|ToString(Integer) Num))
  (Variables|Default|SetNumString (select (Utilities|Array|IsEmpty (Variables|Default|GetNumString)) _returnvalue (Utilities|String|Append (Variables|Default|GetNumString) _returnvalue)))
  (CallFunction|UpdateDisplay))

(event Custom|UpdateDisplay
  (bind _aswbp_display_number (Utilities|Casting|CastToWBP_DisplayNumber (UserInterface|GetWidget (Variables|Default|GetWidget))))
  (Default|SetNumber _aswbp_display_number (Math|Conversions|ToInteger(Byte) (Variables|Default|GetNumString)))
  (if (>= (Utilities|String|Len (Variables|Default|GetNumString)) 4)
    (bind _returnvalue (Actor|GetActorOfClass "/Game/Blueprints/Levels/GameplayLevel/BP_PuzzleGameplay.BP_PuzzleGameplay_C"))
    (if (== (Variables|/Game/Blueprints/Levels/GameplayLevel/BP_PuzzleGameplay.BP_PuzzleGameplay_C|GetDisplayNumber _returnvalue) (Math|Conversions|ToInteger(Byte) (Variables|Default|GetNumString)))
      (Development|PrintString "YOU WIN!!!")
      (Default|OpenEndDoor _returnvalue)
      (else
        (Variables|Default|SetNumString "")
        (CallFunction|UpdateDisplay)))))

(event EventBeginPlay
  (for _array_element (Utilities|Array|MakeArray (Variables|Default|GetChildActor4) (Variables|Default|GetChildActor2) (Variables|Default|GetChildActor1) (Variables|Default|GetChildActor) (Variables|Default|GetChildActor3) (Variables|Default|GetChildActor8) (Variables|Default|GetChildActor7) (Variables|Default|GetChildActor6) (Variables|Default|GetChildActor5) (Variables|Default|GetChildActor9))
    (bind _asbp_keypad_num (Utilities|Casting|CastToBP_KeypadNum (Variables|/Script/Engine.ChildActorComponent|GetChildActor _array_element)))
    (EventDispatchers|AssignOnKeyPressed _asbp_keypad_num (EventDispatchers|CreateEvent :!event Custom|OnKeyPressed_Event))))

(fn ConstructionScript)