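; Puzzle gameplay Blueprint for the gameplay level that holds a replicated code number and opens the end door.
; On BeginPlay the authority picks a random four-digit DisplayNumber, and its RepNotify calls OnDisplayNumberChanged so listeners can react.
; The OpenEndDoor event extends the parent's handling by finding a BP_ExitDoor in the world and destroying it.
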(event EventBeginPlay
  (|CallParentFunction)
  (if (Ability|HasAuthority)
    (Variables|Default|SetDisplayNumber (Math|Random|RandomIntegerinRange 1000 9999))))

(event EventOpenEndDoor
  (|CallParentFunction)
  (bind _returnvalue (Actor|GetActorOfClass "/Game/Blueprints/Levels/GameplayLevel/BP_ExitDoor.BP_ExitDoor_C"))
  (Utilities|IsValid _returnvalue
    (:Is%20Valid
      (Actor|DestroyActor _returnvalue))))

(fn ConstructionScript
  (|CallParentFunction))

(fn OnRepDisplayNumber
  (Default|CallOnDisplayNumberChanged))