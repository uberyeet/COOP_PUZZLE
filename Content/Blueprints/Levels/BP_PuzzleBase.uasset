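; Base puzzle Blueprint that detects when players reach a level end box and signals that the puzzle is complete.
; On BeginPlay it binds to the reached and left events of each LevelEndBox, or prints a warning if none exist.
; These events maintain a player count, and a reach that brings it to at least one calls CompletePuzzle, which broadcasts OnPuzzleCompleted.
; OpenEndDoor is an empty event here.
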(event Custom|OnLevelEndBoxReached_Event
  (bind _result (Math|Integer|IncrementInt (Variables|Default|GetPlayersOnEndBox))
    (:%20%20
      (if (>= _result 1)
        (CallFunction|CompletePuzzle)))))

(event Custom|OpenEndDoor)

(event Custom|OnLevelEndBoxLeft_Event
  (Math|Integer|DecrementInt (Variables|Default|GetPlayersOnEndBox)))

(event EventBeginPlay
  (if (Utilities|Array|IsNotEmpty (Variables|Default|GetLevelEndBoxes))
    (for _array_element (Variables|Default|GetLevelEndBoxes)
      (EventDispatchers|AssignOnLevelEndBoxReached _array_element (delegate Custom|OnLevelEndBoxReached_Event))
      (EventDispatchers|AssignOnLevelEndBoxLeft _array_element (delegate Custom|OnLevelEndBoxLeft_Event)))
    (else
      (Development|PrintString "PUZZLE HAS NO END BOXES"))))

(fn ConstructionScript)

(fn CompletePuzzle
  (Default|CallOnPuzzleCompleted))