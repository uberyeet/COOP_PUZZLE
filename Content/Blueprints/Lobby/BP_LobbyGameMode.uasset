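; BP_LobbyGameMode is the lobby game mode that tracks joining players and starts the match.
; PostLogin adds each lobby player controller to a list and, for the first two, sends a role message to its PlayerState based on join order.
; Logout removes the controller from the list.
; StartMatch server-travels everyone to the gameplay map; an older console-command travel is left unconnected.
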(event EventPostLogin
  (params (NewPlayer :type Player%20Controller%20Object%20Reference))
  (bind _pcs (Variables|Default|GetPCs))
  (bind _asbp_lobby_player_controller (Utilities|Casting|CastToBP_LobbyPlayerController NewPlayer))
  (Utilities|Array|Add _pcs _asbp_lobby_player_controller)
  (switch int (Utilities|Array|Length _pcs)
    (:1
      (Class|BPIPlayerInformation|SetRole(Message) (Variables|/Script/Engine.Controller|GetPlayerState _asbp_lobby_player_controller) "NewEnumerator0"))
    (:2
      (Class|BPIPlayerInformation|SetRole(Message) (Variables|/Script/Engine.Controller|GetPlayerState _asbp_lobby_player_controller) "NewEnumerator1"))))

(event EventOnLogout
  (params (ExitingController :type Controller%20Object%20Reference))
  (bind _asbp_lobby_player_controller (Utilities|Casting|CastToBP_LobbyPlayerController ExitingController))
  (Utilities|Array|RemoveItem (Variables|Default|GetPCs) _asbp_lobby_player_controller))

(fn ConstructionScript)

(fn StartMatch
  (Class|AdvancedSessionsLibrary|ServerTravel "L_GameplayMap" false false))