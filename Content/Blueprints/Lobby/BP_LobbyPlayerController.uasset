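; Lobby player controller that drives the local player's lobby UI and ready state.
; On BeginPlay, the local controller creates the lobby widget, shows the cursor and sets Game and UI input.
; Events toggle Ready on the lobby PlayerState and reveal the widget's animated loading screen.
; The 1 key prints the player's role message as a debug readout.
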(event Custom|ReadyUp
  (bind _asbp_lobby_player_state (Utilities|Casting|CastToBP_LobbyPlayerState (Variables|GetPlayerState)))
  (Variables|/Game/Blueprints/Lobby/BP_LobbyPlayerState.BP_LobbyPlayerState_C|SetbReady _asbp_lobby_player_state (not (Variables|/Game/Blueprints/Lobby/BP_LobbyPlayerState.BP_LobbyPlayerState_C|GetbReady _asbp_lobby_player_state))))

(event Custom|LoadingScreen
  (bind _lobbyui (Variables|Default|GetLobbyUI))
  (Widget|SetVisibility (Variables|/Game/Blueprints/Lobby/WBP_LobbyUI.WBP_LobbyUI_C|GetWBP_LoadingScreen _lobbyui) "Visible")
  (UserInterface|Animation|PlayAnimation _lobbyui (Variables|/Game/Blueprints/Lobby/WBP_LobbyUI.WBP_LobbyUI_C|GetLoadingScreenAnim _lobbyui) 0.0 1 "Forward" 1.0 false))

(event EventBeginPlay
  (if (Pawn|IsLocalPlayerController)
    (Utilities|FlowControl|Sequence
      (:then_0
        ;[0.15 0.15 0.15 0.5] Widget
        (bind _returnvalue (UserInterface|CreateWidget "/Game/Blueprints/Lobby/WBP_LobbyUI.WBP_LobbyUI_C"))
        (Variables|Default|SetLobbyUI _returnvalue)
        (UserInterface|Viewport|AddtoViewport _returnvalue 0)
        (Variables|Default|SetbShowMouseCursor true)
        (Input|SetInputModeGameandUI self 0 "DoNotLock" true false)))))

(event Input|KeyboardEvents|1
  (params (Key :type Key%20Structure :default "None"))
  (:Pressed
    (bind _role (Class|BPIPlayerInformation|GetRole(Message) (Variables|GetPlayerState)))
    (Development|PrintString (Utilities|String|EnumtoString _role))))

(fn ConstructionScript)