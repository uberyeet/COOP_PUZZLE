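; BP_Button is an interactable button that toggles the visibility of its Sphere when used.
; Interact forwards the Role to MC_Interact, apparently a multicast by its name, which flips the sphere and prints the role.
; Query functions report it as always interactable and never edible, with instant interaction followed by a short cooldown.
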(event Custom|MC_Interact
  (params (Role :type E_Roles%20Enum :default "NewEnumerator0"))
  (bind _sphere (Variables|Default|GetSphere))
  (Rendering|SetVisibility _sphere (not (Variables|/Script/Engine.SceneComponent|GetbVisible _sphere)) false)
  (Development|PrintString (Utilities|String|EnumtoString Role)))

(event EventInteract
  (params (Interactor :type Actor%20Object%20Reference) (Role :type E_Roles%20Enum :default "NewEnumerator0"))
  (CallFunction|MCInteract Role))

(fn ConstructionScript)

(fn CanbeEaten?
  (return false))

(fn CanInteract?
  (return true))

(fn InteractCooldown
  (return 2.0))

(fn InteractTime
  (return 0.0))